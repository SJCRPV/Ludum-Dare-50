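; AdorableMagician_BP is a player-controlled pawn or character that moves within the X–Z plane, as in a side-view game.
; Four axis inputs (left, right, up, down) each feed AddMovementInput along a fixed world axis, scaled by a Speed variable.
; Vertical movement input is forced, while horizontal input is not.
; BeginPlay, overlap, Tick and the construction script contain no logic.
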(event EventBeginPlay)

(event Collision|EventActorBeginOverlap
  (params (OtherActor :type Actor%20Object%20Reference)))

(event EventTick
  (params (DeltaSeconds :type Float%20%28single-precision%29)))

(event Input|AxisEvents|InputAxisMoveCharacterLeft
  (params (AxisValue :type Float%20%28single-precision%29))
  (Pawn|Input|AddMovementInput "-1.000000, 0, 0" (* AxisValue (Variables|Default|GetSpeed)) false))

(event Input|AxisEvents|InputAxisMoveCharacterRight
  (params (AxisValue :type Float%20%28single-precision%29))
  (Pawn|Input|AddMovementInput "1.000000, 0, 0" (* AxisValue (Variables|Default|GetSpeed)) false))

(event Input|AxisEvents|InputAxisMoveCharacterUp
  (params (AxisValue :type Float%20%28single-precision%29))
  (Pawn|Input|AddMovementInput "0.000000,0.000000,1.000000" (* AxisValue (Variables|Default|GetSpeed)) true))

(event Input|AxisEvents|InputAxisMoveCharacterDown
  (params (AxisValue :type Float%20%28single-precision%29))
  (Pawn|Input|AddMovementInput "0.000000,-0.000000,-1.000000" (* AxisValue (Variables|Default|GetSpeed)) true))

(fn ConstructionScript)