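; Minigame station actor that launches a minigame and shows its UI when something overlaps it.
; On BeginPlay it adds the user widget from its MinigameWidget component to the viewport and hides it.
; On overlap, StartMinigameIfPossible starts the minigame and reveals the widget only if IsNextMinigame is set.
; Every overlap also enables input for player controller 0 and prints a debug greeting, without checking the overlapping actor.
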(event EventBeginPlay
  (bind _minigamewidget (Variables|Default|GetMinigameWidget))
  (bind _returnvalue (UserInterface|GetUserWidgetObject _minigamewidget))
  (if (Utilities|IsValid _returnvalue)
    (UserInterface|Viewport|AddtoViewport _returnvalue 1)
    (Widget|SetVisibility _returnvalue "Hidden")))

(event Collision|EventActorBeginOverlap
  (params (OtherActor :type Actor%20Object%20Reference))
  (CallFunction|StartMinigameifPossible)
  (Input|EnableInput (Game|GetPlayerController 0))
  (Development|PrintText "Hello"))

(event EventTick
  (params (DeltaSeconds :type Float%20%28single-precision%29)))

(fn ConstructionScript)

(fn StartMinigameifPossible
  (if (Variables|MinigameStation|GetIsNextMinigame)
    (Class|Minigame|StartMinigame)
    (Widget|SetVisibility (UserInterface|GetUserWidgetObject (Variables|Default|GetMinigameWidget)) "Visible")))