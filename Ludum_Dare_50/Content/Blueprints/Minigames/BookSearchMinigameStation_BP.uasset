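; Minigame station for a book search puzzle, where the player hunts for the correct page.
; Overlap starts the BookSearch child actor's minigame; BeginPlay passes page content to the widget and binds its slider.
; Page-flip inputs and slider changes recolour a proximity indicator by distance from the correct page.
; Only flips check for an exact match, which wins the minigame and hides the widget.
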(event Custom|OnValueChanged_Event
  (params (Value :type Float%20%28single-precision%29))
  (bind _asbook_search (Utilities|Casting|CastToBookSearch (Variables|/Script/Engine.ChildActorComponent|GetChildActor (Variables|Default|GetMinigameClass))))
  (bind _returnvalue (Class|BookSearch|GetCorrectPage _asbook_search))
  (Class|BookSearchWidget|UpdateColourOfProximityImage (stale EventBeginPlay _asbook_search_wbp) (Math|Integer|Absolute(Integer) (- (Math|Conversions|ToInteger(Byte) (Class|KismetMathLibrary|Round64 (Variables|/Script/Ludum_Dare_50.BookSearchWidget|GetpreviousRecordedPageNumber (stale EventBeginPlay _asbook_search_wbp)))) _returnvalue))))

(event EventBeginPlay
  (|CallParentFunction)
  ;[1 1 1] Bind OnValueChanged Event for the slider, so we can update the proximity sensor
  (bind _asbook_search_wbp (Utilities|Casting|CastToBookSearch_WBP (UserInterface|GetUserWidgetObject (Variables|Default|GetMinigameWidget))))
  (EventDispatchers|AssignOnValueChanged (Variables|/Script/Ludum_Dare_50.BookSearchWidget|GetBookPageSlider _asbook_search_wbp) (delegate Custom|OnValueChanged_Event))
  (Variables|/Script/Ludum_Dare_50.BookSearchWidget|SetgibberishPages _asbook_search_wbp (Variables|Default|GetGibberishPages))
  (Variables|/Script/Ludum_Dare_50.BookSearchWidget|SetclearTextPages _asbook_search_wbp (Variables|Default|GetClearTextPages)))

(event Collision|EventActorBeginOverlap
  (params (OtherActor :type Actor%20Object%20Reference))
  (|CallParentFunction OtherActor)
  (bind _asbook_search (Utilities|Casting|CastToBookSearch (Variables|/Script/Engine.ChildActorComponent|GetChildActor (Variables|Default|GetMinigameClass))))
  (Class|Minigame|StartMinigame _asbook_search))

(event EventTick
  (params (DeltaSeconds :type Float%20%28single-precision%29))
  (|CallParentFunction DeltaSeconds) ; This node is disabled and will not be called.\nDrag off pins to build functionality.
)

(event Input|ActionEvents|InputActionFlipSingleBookPageForward
  (params (Key :type Key%20Structure :default "None"))
  (:Pressed
    (bind _asbook_search_wbp (Utilities|Casting|CastToBookSearch_WBP (UserInterface|GetUserWidgetObject (Variables|Default|GetMinigameWidget))))
    (Default|TurnPageForward _asbook_search_wbp)
    (bind _asbook_search (Utilities|Casting|CastToBookSearch (Variables|/Script/Engine.ChildActorComponent|GetChildActor (Variables|Default|GetMinigameClass))))
    (bind _returnvalue (Class|BookSearch|GetCorrectPage _asbook_search))
    (Class|BookSearchWidget|UpdateColourOfProximityImage _asbook_search_wbp (Math|Integer|Absolute(Integer) (- _returnvalue (Math|Conversions|ToInteger(Byte) (Class|KismetMathLibrary|Round64 (Variables|/Script/Ludum_Dare_50.BookSearchWidget|GetpreviousRecordedPageNumber _asbook_search_wbp))))))
    (Math|Integer|CompareInt (Math|Integer|Absolute(Integer) (- _returnvalue (Math|Conversions|ToInteger(Byte) (Class|KismetMathLibrary|Round64 (Variables|/Script/Ludum_Dare_50.BookSearchWidget|GetpreviousRecordedPageNumber _asbook_search_wbp)))))
      (:==
        (Class|Minigame|WinMinigame (stale Input|ActionEvents|InputActionFlipSingleBookPageBackward _asbook_search))
        (bind _asbook_search_wbp_2 (Utilities|Casting|CastToBookSearch_WBP (UserInterface|GetUserWidgetObject (Variables|Default|GetMinigameWidget))))
        (Widget|SetVisibility _asbook_search_wbp_2 "Hidden")))))

(event Input|ActionEvents|InputActionFlipSingleBookPageBackward
  (params (Key :type Key%20Structure :default "None"))
  (:Pressed
    (bind _asbook_search_wbp (Utilities|Casting|CastToBookSearch_WBP (UserInterface|GetUserWidgetObject (Variables|Default|GetMinigameWidget))))
    (Default|TurnPageBack _asbook_search_wbp)
    (bind _asbook_search (Utilities|Casting|CastToBookSearch (Variables|/Script/Engine.ChildActorComponent|GetChildActor (Variables|Default|GetMinigameClass))))
    (bind _returnvalue (Class|BookSearch|GetCorrectPage _asbook_search))
    (Class|BookSearchWidget|UpdateColourOfProximityImage _asbook_search_wbp (Math|Integer|Absolute(Integer) (- (Math|Conversions|ToInteger(Byte) (Class|KismetMathLibrary|Round64 (Variables|/Script/Ludum_Dare_50.BookSearchWidget|GetpreviousRecordedPageNumber _asbook_search_wbp))) _returnvalue)))
    (Math|Integer|CompareInt (Math|Integer|Absolute(Integer) (- (Math|Conversions|ToInteger(Byte) (Class|KismetMathLibrary|Round64 (Variables|/Script/Ludum_Dare_50.BookSearchWidget|GetpreviousRecordedPageNumber _asbook_search_wbp))) _returnvalue))
      (:==
        (Class|Minigame|WinMinigame _asbook_search)
        (bind _asbook_search_wbp_2 (Utilities|Casting|CastToBookSearch_WBP (UserInterface|GetUserWidgetObject (Variables|Default|GetMinigameWidget))))
        (Widget|SetVisibility _asbook_search_wbp_2 "Hidden")))))

(fn ConstructionScript
  (|CallParentFunction))