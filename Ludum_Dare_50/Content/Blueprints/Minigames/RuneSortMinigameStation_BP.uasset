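; RuneSortMinigameStation_BP is a minigame station that launches the rune sorting minigame when an actor overlaps it.
; On overlap it runs the parent handler, then checks whether it is flagged as the next minigame.
; If so, it casts the child actor of its MinigameClass component to RuneSorter and calls StartMinigame on it.
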(event EventBeginPlay
  (|CallParentFunction) ; This node is disabled and will not be called.\nDrag off pins to build functionality.
)

(event Collision|EventActorBeginOverlap
  (params (OtherActor :type Actor%20Object%20Reference))
  (|CallParentFunction OtherActor)
  (if (Variables|Default|GetIsNextMinigame)
    (bind _asrune_sorter (Utilities|Casting|CastToRuneSorter (Variables|/Script/Engine.ChildActorComponent|GetChildActor (Variables|Default|GetMinigameClass))))
    (Class|Minigame|StartMinigame _asrune_sorter)))

(event EventTick
  (params (DeltaSeconds :type Float%20%28single-precision%29))
  (|CallParentFunction DeltaSeconds) ; This node is disabled and will not be called.\nDrag off pins to build functionality.
)

(fn ConstructionScript
  (|CallParentFunction))